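; Master death zone actor that triggers the player's death screen when BP_Player enters its box.
; On overlap it spawns a Niagara death effect at the player, plays a 2D death sound and pauses the game after a short delay.
; It then shows the WIB_Death widget with UI-only input focused on its continue button, removes the player's two HUD widgets and hides the player mesh.
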(event OnComponentBeginOverlap(Box)
  (params (OverlappedComponent :type Primitive%20Component%20Object%20Reference) (OtherActor :type Actor%20Object%20Reference) (OtherComp :type Primitive%20Component%20Object%20Reference) (OtherBodyIndex :type Integer) (bFromSweep :type Boolean) (SweepResult :type Hit%20Result%20Structure%20%28by%20ref%29))
  (bind _asbp_player (Utilities|Casting|CastToBP_Player OtherActor))
  (Variables|/Game/Blueprints/Character/BP_Player.BP_Player_C|SetIsDeath? _asbp_player false)
  (Niagara|SpawnSystematLocation "/Game/VFX/NiagaraSysteme/DeathVariante/NS_Death_Yellow.NS_Death_Yellow" (Transformation|GetWorldLocation (Variables|/Script/Engine.Actor|GetRootComponent _asbp_player)))
  (Audio|PlaySound2D "/Game/Sound/SFX/Player/death.death" 1.0 1.0 0.0 0 0)
  (Utilities|FlowControl|Delay 0.3)
  (Game|SetGamePaused true)
  (bind _returnvalue (UserInterface|CreateWidget "/Game/Widget/WIB_Death.WIB_Death_C"))
  (UserInterface|Viewport|AddtoViewport _returnvalue 0)
  (Input|SetInputModeUIOnly (Game|GetPlayerController 0) (Variables|/Game/Widget/WIB_Death.WIB_Death_C|GetBtn_Continue _returnvalue) "DoNotLock" false)
  (Utilities|FlowControl|Sequence
    (:then_0
      (bind _hud_ref (Variables|/Game/Blueprints/Character/BP_Player.BP_Player_C|GetHUD_Ref _asbp_player)
        (:then
          (Widget|RemovefromParent _hud_ref))
        (:else)))
    (:then_1
      (bind _oeuf_hud_ref (Variables|/Game/Blueprints/Character/BP_Player.BP_Player_C|GetOeuf_HUD_Ref _asbp_player)
        (:then
          (Widget|RemovefromParent _oeuf_hud_ref))
        (:else)))
    (:then_2
      (Rendering|SetVisibility (Variables|/Script/Engine.Character|GetMesh _asbp_player) false false))))

(event EventBeginPlay)

(event Collision|EventActorBeginOverlap
  (params (OtherActor :type Actor%20Object%20Reference)))

(event EventTick
  (params (DeltaSeconds :type Float%20%28single-precision%29)))

(fn ConstructionScript)