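; Air current volume (Drought) that pushes BP_Player along its Arrow direction while the player is inside the Box.
; On entry it registers itself on the player and, unless deflated, zeroes velocity and gravity; exit calls SetCharacterMovement.
; A looping timer repeatedly launches non-deflated players, with strength depending on inflation, standstill and volume Rotation.
; The construction script applies Dimensions and Rotation to the Box and Niagara effect.
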(event OnComponentBeginOverlap(Box)
  (params (OverlappedComponent :type Primitive%20Component%20Object%20Reference) (OtherActor :type Actor%20Object%20Reference) (OtherComp :type Primitive%20Component%20Object%20Reference) (OtherBodyIndex :type Integer) (bFromSweep :type Boolean) (SweepResult :type Hit%20Result%20Structure%20%28by%20ref%29))
  (bind _asbp_player (Utilities|Casting|CastToBP_Player OtherActor))
  (Variables|Default|SetAs%20BP%20Player _asbp_player)
  (if (Variables|/Game/Blueprints/Character/BP_Player.BP_Player_C|GetIsDeflates? _asbp_player)
    (Variables|/Game/Blueprints/Character/BP_Player.BP_Player_C|SetIsInDrought? _asbp_player true)
    (Variables|/Game/Blueprints/Character/BP_Player.BP_Player_C|SetRef_Drought _asbp_player self)
    (Variables|Default|SetIs_In_Drought? true)
    (else
      (Variables|/Game/Blueprints/Character/BP_Player.BP_Player_C|SetIsInDrought? _asbp_player true)
      (Variables|/Game/Blueprints/Character/BP_Player.BP_Player_C|SetRef_Drought _asbp_player self)
      (Variables|/Script/Engine.MovementComponent|SetVelocity (Variables|/Script/Engine.Character|GetCharacterMovement _asbp_player) "0, 0, 0")
      (Variables|/Script/Engine.CharacterMovementComponent|SetGravityScale (Variables|/Script/Engine.Character|GetCharacterMovement _asbp_player) 0.0)
      (Variables|Default|SetIs_In_Drought? true))))

(event OnComponentEndOverlap(Box)
  (params (OverlappedComponent :type Primitive%20Component%20Object%20Reference) (OtherActor :type Actor%20Object%20Reference) (OtherComp :type Primitive%20Component%20Object%20Reference) (OtherBodyIndex :type Integer))
  (Variables|Default|SetIs_In_Drought? false)
  (Variables|Default|GetAs%20BP%20Player
    (:then
      (Default|SetCharacterMovement (Variables|Default|GetAs%20BP%20Player)))
    (:else)))

(event Custom|UpdateVelocity
  (if (Variables|Default|GetIs_In_Drought?)
    (bind _as_bp_player (Variables|Default|GetAs%20BP%20Player)
      (:then
        (if (not (Variables|/Game/Blueprints/Character/BP_Player.BP_Player_C|GetIsDeflates? _as_bp_player))
          (if (Variables|/Game/Blueprints/Character/BP_Player.BP_Player_C|GetIsInflate? _as_bp_player)
            (if (Utilities|Operators|EqualEqual :A (Transformation|GetVelocity (Variables|Default|GetAs%20BP%20Player)))
              (Character|LaunchCharacter (Variables|Default|GetAs%20BP%20Player) (* (Math|Vector|GetForwardVector (Variables|Default|GetArrow)) "1500.000000,1500.000000,500.000000") false false)
              (elif (Utilities|Operators|EqualEqual :A (Variables|Default|GetRotation))
                (Character|LaunchCharacter (Variables|Default|GetAs%20BP%20Player) (* (Math|Vector|GetForwardVector (Variables|Default|GetArrow)) "150.000000,150.000000,150.000000") false false)
                (else
                  (Character|LaunchCharacter (Variables|Default|GetAs%20BP%20Player) (* (Math|Vector|GetForwardVector (Variables|Default|GetArrow)) "850.000000,850.000000,850.000000") false false))))
            (elif (Utilities|Operators|EqualEqual :A (Transformation|GetVelocity (Variables|Default|GetAs%20BP%20Player)))
              (Character|LaunchCharacter (Variables|Default|GetAs%20BP%20Player) (* (Math|Vector|GetForwardVector (Variables|Default|GetArrow)) "1500.000000,1500.000000,500.000000") false false)
              (elif (Utilities|Operators|EqualEqual :A (Variables|Default|GetRotation))
                (Character|LaunchCharacter (Variables|Default|GetAs%20BP%20Player) (* (Math|Vector|GetForwardVector (Variables|Default|GetArrow)) "150.000000,150.000000,150.000000") false false)
                (else
                  (Character|LaunchCharacter (Variables|Default|GetAs%20BP%20Player) (* (Math|Vector|GetForwardVector (Variables|Default|GetArrow)) "1000.000000,1000.000000,1000.000000") false false)))))))
      (:else))))

(event EventBeginPlay
  (Utilities|Time|SetTimerbyEvent (delegate Custom|UpdateVelocity) 0.2 true))

(fn ConstructionScript
  (bind _box (Variables|Default|GetBox))
  (if (not (Utilities|Operators|NotEqual(!=) (Transformation|GetActorScale3D) "1.000000,1.000000,1.000000" 0.0))
    (Transformation|SetActorScale3D "1.000000,1.000000,1.000000")
    (Transformation|SetActorRotation (Math|Rotator|MakeRotator 0.0 0.0 (.yaw (Transformation|GetActorRotation))))
    (Transformation|SetRelativeLocation _box (Math|Vector|MakeVector 0.0 0.0 (.z (Variables|Default|GetDimensions))) false false)
    (Components|Box|SetBoxExtent _box (Variables|Default|GetDimensions) true)
    (Transformation|SetRelativeRotation (Variables|Default|GetBox) (Variables|Default|GetRotation) false false)
    (Effects|Components|ParticleSystem|SetFloatParameter (Variables|Default|GetNiagara) "Cylinde_Height" (/ (.z (Variables|Default|GetDimensions)) 2.0))
    (Transformation|SetWorldRotation (Variables|Default|GetNiagara) (Variables|Default|GetRotation) false false)))