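; BP_Projectile is an enemy projectile that kills the player on contact.
; Its sphere collision overlap ignores BP_Ennemy actors and, on an exact BP_Player class match, destroys both itself and the player, then removes all widgets.
; Overlaps with any other actor have no effect, and the projectile destroys itself five seconds after BeginPlay.
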(event OnComponentBeginOverlap(SphereCollision)
  (params (OverlappedComponent :type Primitive%20Component%20Object%20Reference) (OtherActor :type Actor%20Object%20Reference) (OtherComp :type Primitive%20Component%20Object%20Reference) (OtherBodyIndex :type Integer) (bFromSweep :type Boolean) (SweepResult :type Hit%20Result%20Structure%20%28by%20ref%29))
  (bind _returnvalue (Utilities|GetClass OtherActor))
  (if (not (== _returnvalue "/Game/Luca/Ennemy/Blueprint/BP_Ennemy.BP_Ennemy_C"))
    (if (== _returnvalue "/Game/Blueprints/Character/BP_Player.BP_Player_C")
      (Actor|DestroyActor)
      (Actor|DestroyActor OtherActor)
      (Viewport|RemoveAllWidgets))))

(event EventBeginPlay
  (Utilities|FlowControl|Delay 5.0)
  (Actor|DestroyActor))

(fn ConstructionScript)