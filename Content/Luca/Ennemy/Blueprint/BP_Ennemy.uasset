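; Flying octopus enemy character that roams around its spawn point, turns toward the player and fires projectiles.
; Passes itself and its AI state to the BB_Ennemy blackboard, and exposes roam, move and chase functions.
; Roam targets respect per-axis locks, whose flags also pick the axis for timer-flipped strafing within attack distance.
; Movement steers by direct input, and an attack montage notify spawns the projectile, effect and sound.
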(event Custom|InvestigateStrafe
  (bind _isa (Utilities|FlowControl|FlipFlop)
    (:A
      _)
    (:B
      _))
  (Variables|Default|SetInvestigateStrafeRight _isa)
  (Utilities|Time|SetTimerbyEvent (delegate Custom|InvestigateStrafe) 5.0))

(event Custom|CheckAndFire
  (CallFunction|FindLookatPlayer)
  (if (not (Variables|Default|GetIsDead))
    (CallFunction|FireEffetcs)
    (Utilities|FlowControl|Delay (Variables|SettingsAttack|GetDelayAttack))
    (Variables|Default|SetIsFiring false)))

(event Custom|FireEffetcs
  (bind _mesh (Variables|Character|GetMesh))
  (bind _returnvalue (Transformation|GetSocketTransform _mesh "joint2" "RTS_World"))
  (bind _notifyname (Animation|Montage|PlayMontage (Variables|Character|GetMesh) "/Game/Luca/Ennemy/Assets/AM_poulpiattack.AM_poulpiattack" 1.5)
    (:OnNotifyBegin
      (if (== _notifyname "Attack")
        (Niagara|SpawnSystematLocation "/Game/VFX/NiagaraSysteme/NS_AttackPoulpe.NS_AttackPoulpe" (.location (Transformation|GetSocketTransform (Variables|Character|GetMesh) "joint2" "RTS_World")) (Transformation|GetActorRotation) "10.000000,10.000000,10.000000")
        (Game|SpawnActorfromClass (Variables|SettingsAttack|GetProjectille) (Math|Transform|MakeTransform (.location _returnvalue) (Transformation|GetActorRotation) (.scale _returnvalue)) "AlwaysSpawn" "MultiplyWithRoot" 0 0)
        (Audio|PlaySoundatLocation (Variables|SettingsAttack|GetSFX_Attack) "0, 0, 0" "0, 0, 0" 0.1 1.0 0.0 0 0 0 0)))))

(event Custom|ChaseStrafe
  (bind _isa (Utilities|FlowControl|FlipFlop)
    (:A
      _)
    (:B
      _))
  (Variables|Default|SetChaseStrafeRight _isa)
  (Utilities|Time|SetTimerbyEvent (delegate Custom|ChaseStrafe) 2.0))

(event EventBeginPlay
  (Utilities|FlowControl|Sequence
    (:then_0
      (bind _asaic_ennemy (Utilities|Casting|CastToAIC_Ennemy (Pawn|GetController)))
      (bind _output_get (Variables|Default|SetEnnemyRef _asaic_ennemy))
      (bind _blackboardcomponent (Class|AIController|UseBlackboard _output_get "/Game/Luca/Ennemy/Blueprint/AI/BB_Ennemy.BB_Ennemy"))
      (bind _output_get_2 (Variables|Default|SetBlackboardRef _blackboardcomponent))
      (AI|Components|Blackboard|SetValueasObject _output_get_2 (Utilities|Name|MakeLiteralName "EnnemyActor") self))
    (:then_1
      (bind _output_get_3 (Variables|Default|SetStartLocation (Transformation|GetActorLocation)))
      (Variables|Default|SetPositionWorldStart _output_get_3))
    (:then_2
      (Utilities|Casting|CastToBP_Player (Game|GetPlayerCharacter 0)))
    (:then_3
      (CallFunction|ChaseStrafe)
      (CallFunction|InvestigateStrafe))))

(event EventTick
  (params (DeltaSeconds :type Float%20%28single-precision%29))
  (AI|Components|Blackboard|SetValueasEnum (Variables|Default|GetBlackboardRef) (Utilities|Name|MakeLiteralName "EnnemyState") (Variables|Default|GetAIStates)))

(fn ConstructionScript)

(fn FindLookatPlayer
  (Transformation|SetWorldRotation (Variables|Default|GetArrow1) (Math|Rotator|FindLookatRotation (Transformation|GetWorldLocation (Variables|Default|GetArrow1)) (Transformation|GetSocketLocation (Variables|/Script/Engine.Character|GetMesh (Variables|Default|GetPlayerReference)) "joint1")) false false))

(fn ChasePlayer
  (bind _chasestraferight (Variables|Default|GetChaseStrafeRight))
  (bind _returnvalue (Math|Float|SelectFloat -0.5 0.5 _chasestraferight))
  (switch Utilities|FlowControl|Switch|SwitchonChase_States (Variables|Default|GetChaseState)
    (:NewEnumerator0
      (if (> (Transformation|GetDistanceTo (Variables|Default|GetPlayerReference)) (Variables|SettingsAttack|GetAttackDistance))
        (bind _asbp_player (Utilities|Casting|CastToBP_Player (Game|GetPlayerCharacter 0) :!label _label))
        (Variables|Default|SetPlayerReference _asbp_player)
        (if (Variables|Default|GetIsFiring)
          (Transformation|SetActorRotation (Math|Rotator|Lerp(Rotator) (Transformation|GetActorRotation) (Math|Rotator|MakeRotator (.roll (Math|Rotator|FindLookatRotation (Transformation|GetActorLocation) (Math|Vector|MakeVector (.x (Transformation|GetActorLocation (Variables|Default|GetPlayerReference))) (.y (Transformation|GetActorLocation (Variables|Default|GetPlayerReference))) (.z (Transformation|GetActorLocation (Variables|Default|GetPlayerReference)))))) (.pitch (Math|Rotator|FindLookatRotation (Transformation|GetActorLocation) (Math|Vector|MakeVector (.x (Transformation|GetActorLocation (Variables|Default|GetPlayerReference))) (.y (Transformation|GetActorLocation (Variables|Default|GetPlayerReference))) (.z (Transformation|GetActorLocation (Variables|Default|GetPlayerReference)))))) (.yaw (Math|Rotator|FindLookatRotation (Transformation|GetActorLocation) (Math|Vector|MakeVector (.x (Transformation|GetActorLocation (Variables|Default|GetPlayerReference))) (.y (Transformation|GetActorLocation (Variables|Default|GetPlayerReference))) (.z (Transformation|GetActorLocation (Variables|Default|GetPlayerReference))))))) 0.2 true))
          (return false)
          (else
            (Variables|Default|SetIsFiring true)
            (CallFunction|CheckandFire)))
        (elif (Variables|CasDeplacement|GetCasXYZ)
          (Pawn|Input|AddMovementInput (Class|KismetMathLibrary|RandomUnitVectorinConeinRadians "10.000000,10.000000,10.000000" 0.0) _returnvalue false)
          (goto _label)
          (elif (Variables|CasDeplacement|GetCasYZ)
            (Pawn|Input|AddMovementInput (Class|KismetMathLibrary|RandomUnitVectorinConeinRadians "0.000000,10.000000,10.000000" 0.0) _returnvalue false)
            (goto _label)
            (elif (Variables|CasDeplacement|GetCasXZ)
              (Pawn|Input|AddMovementInput (Class|KismetMathLibrary|RandomUnitVectorinConeinRadians "10.000000,0.000000,10.000000" 0.0) _returnvalue false)
              (goto _label)
              (elif (Variables|CasDeplacement|GetCasXY)
                (Pawn|Input|AddMovementInput (Class|KismetMathLibrary|RandomUnitVectorinConeinRadians "10.000000,10.000000,0.000000" 0.0) _returnvalue false)
                (goto _label)
                (elif (Variables|CasDeplacement|GetCasY)
                  (Pawn|Input|AddMovementInput (Math|Vector|GetRightVector "0, 0, 0") _returnvalue false)
                  (goto _label)
                  (elif (Variables|CasDeplacement|GetCasX)
                    (Pawn|Input|AddMovementInput (Math|Vector|GetForwardVector "0, 0, 0") _returnvalue false)
                    (goto _label)
                    (elif (Variables|CasDeplacement|GetCasZ)
                      (Pawn|Input|AddMovementInput (Math|Vector|GetUpVector "0, 0, 0") _returnvalue false)
                      (goto _label))))))))))))

(fn FindRandomLocation
  (bind _positionworldstart (Variables|Default|GetPositionWorldStart))
  (bind _positionworldstart_2 (Variables|Default|GetPositionWorldStart))
  (bind _positionworldstart_3 (Variables|Default|GetPositionWorldStart))
  (bind _positionworldstart_4 (Variables|Default|GetPositionWorldStart))
  (bind _positionworldstart_5 (Variables|Default|GetPositionWorldStart))
  (bind _positionworldstart_6 (Variables|Default|GetPositionWorldStart))
  (bind _positionworldstart_7 (Variables|Default|GetPositionWorldStart))
  (LocalVariables|Setint 0)
  (Variables|/Script/Engine.CharacterMovementComponent|SetMaxFlySpeed (Variables|Character|GetCharacterMovement self) (Variables|SettingsMoving|GetMax%20Fly%20Speed))
  (if (Variables|SettingsMoving|GetAxeXBlock?) :!label _label
    (if (Variables|SettingsMoving|GetAxeYBlock?)
      (if (Variables|SettingsMoving|GetAxeZBlock?)
        (Variables|Default|SetTargetLocation (Transformation|GetActorLocation))
        (else
          (Variables|Default|SetTargetLocation (Math|Vector|MakeVector (.x _positionworldstart_2) (.y _positionworldstart_2) (+ (.z _positionworldstart_2) (Math|Random|RandomFloatinRange (Variables|SettingsMoving|GetMinZ) (Variables|SettingsMoving|GetMaxZ)))))
          (Variables|CasDeplacement|SetCasZ true)))
      (elif (Variables|SettingsMoving|GetAxeZBlock?)
        (Variables|Default|SetTargetLocation (Math|Vector|MakeVector (.x _positionworldstart_3) (+ (.y _positionworldstart_3) (Math|Random|RandomFloatinRange (Variables|SettingsMoving|GetMinY) (Variables|SettingsMoving|GetMaxY))) (.z _positionworldstart_3)))
        (Variables|CasDeplacement|SetCasY true)
        (else
          (Variables|Default|SetTargetLocation (Math|Vector|MakeVector (.x _positionworldstart_4) (+ (.y _positionworldstart_4) (Math|Random|RandomFloatinRange (Variables|SettingsMoving|GetMinY) (Variables|SettingsMoving|GetMaxY))) (+ (.z _positionworldstart_4) (Math|Random|RandomFloatinRange (Variables|SettingsMoving|GetMinZ) (Variables|SettingsMoving|GetMaxZ)))))
          (Variables|CasDeplacement|SetCasYZ true))))
    (elif (Variables|SettingsMoving|GetAxeYBlock?)
      (if (Variables|SettingsMoving|GetAxeZBlock?)
        (Variables|Default|SetTargetLocation (Math|Vector|MakeVector (+ (.x _positionworldstart_5) (Math|Random|RandomFloatinRange (Variables|SettingsMoving|GetMinX) (Variables|SettingsMoving|GetMaxX))) (.y _positionworldstart_5) (.z _positionworldstart_5)))
        (Variables|CasDeplacement|SetCasX true)
        (else
          (Variables|Default|SetTargetLocation (Math|Vector|MakeVector (+ (.x _positionworldstart_6) (Math|Random|RandomFloatinRange (Variables|SettingsMoving|GetMinX) (Variables|SettingsMoving|GetMaxX))) (.y _positionworldstart_6) (+ (.z _positionworldstart_6) (Math|Random|RandomFloatinRange (Variables|SettingsMoving|GetMinZ) (Variables|SettingsMoving|GetMaxZ)))))
          (Variables|CasDeplacement|SetCasXZ true)))
      (elif (Variables|SettingsMoving|GetAxeZBlock?)
        (Variables|Default|SetTargetLocation (Math|Vector|MakeVector (+ (.x _positionworldstart_7) (Math|Random|RandomFloatinRange (Variables|SettingsMoving|GetMinX) (Variables|SettingsMoving|GetMaxX))) (+ (.y _positionworldstart_7) (Math|Random|RandomFloatinRange (Variables|SettingsMoving|GetMinY) (Variables|SettingsMoving|GetMaxY))) (.z _positionworldstart_7)))
        (Variables|CasDeplacement|SetCasXY true)
        (else
          (Variables|Default|SetTargetLocation (Math|Vector|MakeVector (+ (.x _positionworldstart) (Math|Random|RandomFloatinRange (Variables|SettingsMoving|GetMinX) (Variables|SettingsMoving|GetMaxX))) (+ (.y _positionworldstart) (Math|Random|RandomFloatinRange (Variables|SettingsMoving|GetMinY) (Variables|SettingsMoving|GetMaxY))) (+ (.z _positionworldstart) (Math|Random|RandomFloatinRange (Variables|SettingsMoving|GetMinZ) (Variables|SettingsMoving|GetMaxZ)))))
          (Variables|CasDeplacement|SetCasXYZ true)))))
  (Variables|Default|SetCanRoamRadius (/ (+ (Math|Float|Absolute(Float) (Variables|SettingsMoving|GetMinX)) (Variables|SettingsMoving|GetMaxX)) 2.0))
  (if (> (Math|Float|Absolute(Float) (Math|Vector|VectorLength (- (Variables|Default|GetStartLocation) (Variables|Default|GetTargetLocation)))) (Variables|Default|GetCanRoamRadius))
    (bind _output_get (LocalVariables|Setint (+ (LocalVariables|Getint) 1)))
    (if (< _output_get 10)
      (goto _label)
      (else
        (return (Variables|Default|GetStartLocation))))
    (else
      (return (Variables|Default|GetTargetLocation)))))

(fn MovetoLocation
  (params (MoveToLocation :type Vector :default "0, 0, 0") (Thresold :type Float%20%28double-precision%29))
  (bind _returnvalue (Transformation|GetActorLocation))
  (bind _returnvalue_2 (Math|Rotator|FindLookatRotation _returnvalue MoveToLocation))
  (if (> (Math|Vector|VectorLength (- (Transformation|GetActorLocation) MoveToLocation)) Thresold)
    (Pawn|Input|AddMovementInput (Math|Rotator|GetRotationXVector (Math|Rotator|MakeRotator (.roll _returnvalue_2) (.pitch _returnvalue_2) (.yaw _returnvalue_2))) 1.0 true)
    (Transformation|SetActorRotation (Math|Rotator|Lerp(Rotator) (Transformation|GetActorRotation) (Math|Rotator|MakeRotator 0.0 0.0 (.yaw _returnvalue_2)) 0.1 true))
    (return false)
    (else
      (Components|Movement|StopMovementImmediately (Variables|Character|GetCharacterMovement))
      (return true))))