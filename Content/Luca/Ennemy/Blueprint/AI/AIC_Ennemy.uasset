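; AI controller for the enemy that runs its behavior tree and switches it between Patrol and Attack based on perception of the player.
; Perception updates loop through each stimulus of Player-tagged actors, calling the sight handler only when the updated-actor index is 0.
; Successful sensing saves stimulus and receiver locations and turns Patrol into Attack on the pawn's state; failed sensing reverts Attack to Patrol.
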(event OnPerceptionUpdated(AIPerception)
  (params (UpdatedActors :type Array%20of%20Actor%20Object%20References))
  (for (_array_element _array_index) UpdatedActors
    (if (Actor|ActorHasTag _array_element "Player")
      (bind _info (Class|AIPerceptionComponent|GetActorsPerception (Variables|Default|GetAIPerception) _array_element))
      (for _array_element_2 (.lastsensedstimuli _info)
        (Variables|Default|SetActiveSense _array_element_2)
        (switch int _array_index
          (:0
            (CallFunction|SightSense)))))))

(event Custom|SightSense
  (bind _ennemyref (Variables|Default|GetEnnemyRef))
  (bind _activesense (Variables|Default|GetActiveSense))
  (bind _ennemyref_2 (Variables|Default|GetEnnemyRef))
  (bind (_age _expirationage _strength _stimuluslocation _receiverlocation _tag _bsuccessfullysensed) (Utilities|Struct|BreakAIStimulus _activesense))
  (if _bsuccessfullysensed
    (Variables|Default|SetStimulus%20Location _stimuluslocation)
    (Variables|Default|SetReceiver%20Location _receiverlocation)
    (switch Utilities|FlowControl|Switch|SwitchonEnnemyState (Variables|/Game/Luca/Ennemy/Blueprint/BP_Ennemy.BP_Ennemy_C|GetAIStates _ennemyref_2)
      (:NewEnumerator0
        (Variables|/Game/Luca/Ennemy/Blueprint/BP_Ennemy.BP_Ennemy_C|SetAIStates _ennemyref_2 "NewEnumerator1")))
    (else
      (switch Utilities|FlowControl|Switch|SwitchonEnnemyState (Variables|/Game/Luca/Ennemy/Blueprint/BP_Ennemy.BP_Ennemy_C|GetAIStates _ennemyref)
        (:NewEnumerator1
          (Variables|/Game/Luca/Ennemy/Blueprint/BP_Ennemy.BP_Ennemy_C|SetAIStates _ennemyref "NewEnumerator0"))))))

(event EventBeginPlay
  (AI|RunBehaviorTree "/Game/Luca/Ennemy/Blueprint/AI/BT_Ennemy.BT_Ennemy")
  (bind _asbp_ennemy (Utilities|Casting|CastToBP_Ennemy (Pawn|GetControlledPawn)))
  (Variables|Default|SetEnnemyRef _asbp_ennemy))

(fn ConstructionScript)