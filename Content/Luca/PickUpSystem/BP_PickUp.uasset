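; BP_PickUp is a pickup actor providing the collection logic for eggs (oeufs) and coins.
; UpdateOeufs and UpdateCoin each check that the passed object's class is exactly BP_Player, then increment counters stored in MyGameInstanceEditor, with egg counts clamped per level and overall.
; Both play a 2D sound, spawn the same egg pickup Niagara effect and destroy the actor.
; No event here calls either function.
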(fn ConstructionScript)

(fn UpdateOeufs
  (params (Object :type Object%20Object%20Reference))
  (if (== (Utilities|GetClass Object) "/Game/Blueprints/Character/BP_Player.BP_Player_C")
    (bind _asmy_game_instance_editor (Utilities|Casting|CastToMyGameInstanceEditor (Game|GetGameInstance)))
    (Variables|/Game/Luca/MyGameInstanceEditor.MyGameInstanceEditor_C|SetNbOeufsCurrentLevel _asmy_game_instance_editor (Math|Integer|Clamp(Integer) (+ (Variables|/Game/Luca/MyGameInstanceEditor.MyGameInstanceEditor_C|GetNbOeufsCurrentLevel _asmy_game_instance_editor) 1) 0 3))
    (Variables|/Game/Luca/MyGameInstanceEditor.MyGameInstanceEditor_C|SetNbOeufsRecup _asmy_game_instance_editor (Math|Integer|Clamp(Integer) (+ (Variables|/Game/Luca/MyGameInstanceEditor.MyGameInstanceEditor_C|GetNbOeufsRecup _asmy_game_instance_editor) 1) 0 12))
    (Development|PrintString (Utilities|String|ToString(Integer) (Variables|/Game/Luca/MyGameInstanceEditor.MyGameInstanceEditor_C|GetNbOeufsCurrentLevel _asmy_game_instance_editor)))
    (Audio|PlaySound2D "/Game/Sound/SFX/Player/egg.egg" 1.0 1.0 0.0 0 0)
    (Niagara|SpawnSystematLocation (Variables|Default|GetVFXEggPickUp) "0, 0, 0")
    (Actor|DestroyActor)))

(fn UpdateCoin
  (params (Object :type Object%20Object%20Reference))
  (if (== (Utilities|GetClass Object) "/Game/Blueprints/Character/BP_Player.BP_Player_C")
    (bind _asmy_game_instance_editor (Utilities|Casting|CastToMyGameInstanceEditor (Game|GetGameInstance)))
    (Variables|/Game/Luca/MyGameInstanceEditor.MyGameInstanceEditor_C|SetNbCoin _asmy_game_instance_editor (+ (Variables|/Game/Luca/MyGameInstanceEditor.MyGameInstanceEditor_C|GetNbCoin _asmy_game_instance_editor) 1))
    (Audio|PlaySound2D (Variables|Default|GetSoundPickUp) 1.0 1.0 0.0 0 0)
    (Niagara|SpawnSystematLocation (Variables|Default|GetVFXEggPickUp) "0, 0, 0")
    (Actor|DestroyActor)))